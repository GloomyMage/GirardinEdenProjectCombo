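; BP_AI is a damageable actor with a floating health bar that dies when its HP runs out.
; Point damage lowers HP and pushes it to the WB_HealthBar widget, printing the damage if the actor survives.
; At zero HP or below, the mesh switches to physics simulation and the actor is destroyed after a short delay.
; Tick rotates the health bar widget component toward the player camera manager.
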(event `self.ReceiveBeginPlay`
  (`self.UpdateHealthBar`))

(event `self.ReceiveTick`
  (params (DeltaSeconds :type "Float (single-precision)"))
  (bind _health_bar_widget (`self.Health Bar Widget`))
  (`SceneComponent.K2_SetWorldRotation` _health_bar_widget (`KismetMathLibrary.FindLookAtRotation` (`SceneComponent.K2_GetComponentLocation` _health_bar_widget) (`SceneComponent.K2_GetComponentLocation` (`PlayerCameraManager.TransformComponent` (`GameplayStatics.GetPlayerCameraManager` 0)))) false false))

(event `self.ReceivePointDamage`
  (params (Damage :type "Float (single-precision)") (DamageType :type "DamageType Object Reference") (HitLocation :type "Vector Structure") (HitNormal :type "Vector Structure") (HitComponent :type "PrimitiveComponent Object Reference") (BoneName :type Name) (ShotFromDirection :type "Vector Structure") (InstigatedBy :type "Controller Object Reference") (DamageCauser :type "Actor Object Reference") (HitInfo :type "HitResult Structure (by ref)"))
  (set `self.HP` (- (`self.HP`) Damage))
  (`self.UpdateHealthBar`)
  (if (<= (`self.HP`) 0.0)
    (`PrimitiveComponent.SetSimulatePhysics` (`self.Mesh`) true)
    (`KismetSystemLibrary.Delay` 3.0)
    (`self.K2_DestroyActor`)
    (else
      (`KismetSystemLibrary.PrintString` (`KismetStringLibrary.Conv_DoubleToString` Damage)))))

(fn `UpdateHealthBar`
  (bind _aswb_health_bar (cast `/Game/WB_HealthBar` (`WidgetComponent.GetUserWidgetObject` (`self.Health Bar Widget`))))
  (set `/Game/WB_HealthBar.HP` (`self.HP`) _aswb_health_bar)
  (return))

(fn `UserConstructionScript`)