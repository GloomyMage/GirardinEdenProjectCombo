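; BP_AI is an enemy with HP that reacts to point damage with sound and montages, destroying itself after death.
; A health bar widget receives HP updates and turns toward the player camera each tick.
; Tick maps player distance and, when close, triggers a DoOnce-gated grunt and attack montage, then adds distance-parameterized audio and re-arms after a short delay.
; Completed hit reactions also reset that gate; the attack applies no damage here.
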(event `self.ReceiveBeginPlay`
  (`self.UpdateHealthBar`))

(event `self.ReceivePointDamage`
  (params (Damage :type "Float (single-precision)") (DamageType :type "DamageType Object Reference") (HitLocation :type "Vector Structure") (HitNormal :type "Vector Structure") (HitComponent :type "PrimitiveComponent Object Reference") (BoneName :type Name) (ShotFromDirection :type "Vector Structure") (InstigatedBy :type "Controller Object Reference") (DamageCauser :type "Actor Object Reference") (HitInfo :type "HitResult Structure (by ref)"))
  (set `self.HP` (- (`self.HP`) Damage))
  (`self.UpdateHealthBar`)
  (if (<= (`self.HP`) 0.0)
    (`GameplayStatics.PlaySoundAtLocation` "/Game/SFX/death_10_alex.death_10_alex" (`self.K2_GetActorLocation`) (struct) 1.0 1.0 0.0 null null null null)
    (`AddComponent|NODE_AddNiagaraComponent-0`)
    (`|PlayMontage` (`self.Mesh`) "/Game/Animations/Montages/Death_Montage.Death_Montage"
      (:`OnBlendOut`
        (`self.K2_DestroyActor`)))
    (else
      (`GameplayStatics.PlaySoundAtLocation` "/Game/SFX/damage_5_alex.damage_5_alex" (`self.K2_GetActorLocation`) (struct) 1.0 1.0 0.0 null null null null)
      (`|PlayMontage` (`self.Mesh`) "/Game/Animations/Montages/Hit_Montage.Hit_Montage"
        (:`OnCompleted`
          (goto _label :!via `Reset`))))))

(event `self.ReceiveTick`
  (params (DeltaSeconds :type "Float (single-precision)"))
  (bind _health_bar_widget (`self.Health Bar Widget`))
  (bind _returnvalue (`KismetMathLibrary.MapRangeClamped` (`self.GetDistanceTo` (`GameplayStatics.GetPlayerCharacter` 0)) 100.0 300.0 0.1 1.0))
  (`SceneComponent.K2_SetWorldRotation` _health_bar_widget (`KismetMathLibrary.FindLookAtRotation` (`SceneComponent.K2_GetComponentLocation` _health_bar_widget) (`SceneComponent.K2_GetComponentLocation` (`PlayerCameraManager.TransformComponent` (`GameplayStatics.GetPlayerCameraManager` 0)))) false false)
  (`/Engine/EditorBlueprintResources/StandardMacros.CompareFloat` _returnvalue 1.0
    (:`<`
      (`/Engine/EditorBlueprintResources/StandardMacros.DoOnce` false :!label _label
        (:`Completed`
          (`GameplayStatics.PlaySoundAtLocation` "/Game/SFX/grunting_2_alex.grunting_2_alex" (`self.K2_GetActorLocation`) (struct) 1.0 1.0 0.0 null null null null)
          (`|PlayMontage` (`self.Mesh`) "/Game/Animations/Montages/Enemy_Attack_Montage.Enemy_Attack_Montage"
            (:`OnCompleted`
              (bind _returnvalue_2 (`AddComponent|NODE_AddAudioComponent-0`))
              (`AudioParameterControllerInterface.SetFloatParameter` _returnvalue_2 "None" _returnvalue)
              (`KismetSystemLibrary.Delay` 0.2)
              (goto _label :!via `Reset`))))))))

(fn `UpdateHealthBar`
  (bind _aswb_health_bar (cast `/Game/Widgets/WB_HealthBar` (`WidgetComponent.GetUserWidgetObject` (`self.Health Bar Widget`))))
  (set `/Game/Widgets/WB_HealthBar.HP` (`self.HP`) _aswb_health_bar)
  (return))

(fn `UserConstructionScript`)