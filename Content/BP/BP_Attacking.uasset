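; Anim notify state that gives the player's weapon swing a damage window during attack animations.
; Each tick it sphere-traces for Pawns between the weapon's Start and End sockets, ignoring the player and drawing debug shapes.
; A hit applies point damage from the player's Damage value, with the hit actor itself passed as DamageCauser.
; DamageActor records victims and clears on notify begin, so each actor is damaged once per window.
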(fn `CanDealDamage`
  (params (Actor :type "Actor Object Reference"))
  (returns (ReturnValue :type Boolean))
  (return (not (`KismetArrayLibrary.Array_Contains` (`self.DamageActor`) Actor))))

(fn `Received_NotifyBegin`
  (params (MeshComp :type "SkeletalMeshComponent Object Reference") (Animation :type "AnimSequenceBase Object Reference") (TotalDuration :type "Float (single-precision)") (EventReference :type "AnimNotifyEventReference Structure (by ref)"))
  (returns (ReturnValue :type Boolean))
  (`KismetArrayLibrary.Array_Clear` (`self.DamageActor`))
  (return false))

(fn `Received_NotifyTick`
  (params (MeshComp :type "SkeletalMeshComponent Object Reference") (Animation :type "AnimSequenceBase Object Reference") (FrameDeltaTime :type "Float (single-precision)") (EventReference :type "AnimNotifyEventReference Structure (by ref)"))
  (returns (ReturnValue :type Boolean))
  (bind _asbp_player (cast `/Game/BP/BP_Player` (`ActorComponent.GetOwner` MeshComp)))
  (bind _weapon (`/Game/BP/BP_Player.Weapon` _asbp_player))
  (bind (_outhit _returnvalue) (`KismetSystemLibrary.SphereTraceSingleForObjects` _asbp_player (`SceneComponent.GetSocketLocation` _weapon "Start") (`SceneComponent.GetSocketLocation` _weapon "End") 25.0 (`|MakeArray` "ObjectTypeQuery3" :!type "EObjectTypeQuery Enum") true (`|MakeArray` _asbp_player :!type "Actor Object Reference") "ForDuration" true (struct :`R` 1.0) (struct :`G` 1.0)))
  (if _returnvalue
    (bind (_bblockinghit _binitialoverlap _time _distance _location _impactpoint _normal _impactnormal _physmat _hitactor) (`GameplayStatics.BreakHitResult` _outhit))
    (if (`self.CanDealDamage` _hitactor)
      (`GameplayStatics.ApplyPointDamage` _hitactor (`KismetMathLibrary.Conv_IntToDouble` (`/Game/BP/BP_Player.Damage` _asbp_player)) _location _outhit null _hitactor "/Script/Engine.DamageType")
      (`KismetArrayLibrary.Array_AddUnique` (`self.DamageActor`) _hitactor)
      (return false))))